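; Attachment inventory that stores item classes in a slot array, sized to a configured slot count at BeginPlay after caching the first-person player character.
; Functions add items to the first empty slot, find a matching class, remove or swap entries, and read item info from class defaults.
; Successful changes refresh the affected slots in the player's MainInventory attachment UI through UpdateSlotAtIndex.
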(event `self.ReceiveBeginPlay`
  ;[1 1 1] Cast Player and Resize Slots
  (bind _asbp_first_person_character (cast `/Game/AdvanceWeaponPack/FirstPersonContent/Blueprints/BP_FirstPersonCharacter` (`GameplayStatics.GetPlayerCharacter` 0)))
  (set `self.Player` _asbp_first_person_character)
  (`KismetArrayLibrary.Array_Resize` (`self.Slots`) (`self.AmountOfSlots`)))

(event `UpdateSlotAtIndex`
  (params (Index :type Integer))
  ;[1 1 1] Get From Inventory
  (`/Game/AdvanceWeaponPack/Widget/Inventory/WeaponAttachment_Slot.Update Slot Attachment` (`|GetArrayItem` (`/Game/AdvanceWeaponPack/Widget/Inventory/Inventory_Attachment.Slots` (`/Game/AdvanceWeaponPack/Widget/Inventory/MainInventory.Inventory_Attachment` (`/Game/AdvanceWeaponPack/FirstPersonContent/Blueprints/BP_FirstPersonCharacter.MainInventory` (`self.Player`)))) Index)))

(fn `AddItem`
  (params (`Item Class` :type "/Game/AdvanceWeaponPack/Blueprints/Attachment/BP_BaseAttachment_BP Class Reference"))
  (returns (`Success?` :type Boolean) (Index :type Integer))
  (locals (LocalClass :type "/Game/AdvanceWeaponPack/Blueprints/Attachment/BP_BaseAttachment_BP Class Reference") (FoundIndex :type Integer :default 0))
  (set `local.LocalClass` `Item Class`)
  (bind (_success _index) (`self.SearchEmptySlot`))
  (if _success
    (bind _output_get (set `local.FoundIndex` _index))
    (`KismetArrayLibrary.Array_Set` (`self.Slots`) _output_get (make `/Game/AdvanceWeaponPack/Blueprints/InventorySlot_Struct` (`local.LocalClass`)))
    (`self.UpdateSlotAtIndex` (`local.FoundIndex`))
    (return true (`local.FoundIndex`))))

(fn `GetItemInfoAtIndex`
  (params (Index :type Integer))
  (returns (SlotInfo :type "/Game/AdvanceWeaponPack/Blueprints/Inventory_Struct Structure") (ItemActor :type "/Game/AdvanceWeaponPack/Blueprints/Attachment/BP_BaseAttachment_BP Class Reference"))
  (bind _itemclass (break `/Game/AdvanceWeaponPack/Blueprints/InventorySlot_Struct` (`|GetArrayItem` (`self.Slots`) Index)))
  (return (`.InventoryStruct` (defaults `Object` _itemclass)) _itemclass))

(fn `IsSlotEmpty?`
  (params (Index :type Integer))
  (returns (Empty :type Boolean))
  (return (not (`KismetSystemLibrary.IsValidClass` (`.ItemClass_3_A40736744D9AD799DC31BD8DDFCB6A7A` (break `/Game/AdvanceWeaponPack/Blueprints/InventorySlot_Struct` (`|GetArrayItem` (`self.Slots`) Index)))))))

(fn `RemoveItemAtIndex`
  (params (Index :type Integer))
  (returns (`Success?` :type Boolean))
  (locals (LocalIndex :type Integer))
  (set `local.LocalIndex` Index)
  (if (not (`self.IsSlotEmpty?` (`local.LocalIndex`)))
    (`KismetArrayLibrary.Array_Set` (`self.Slots`) (`local.LocalIndex`) (make `/Game/AdvanceWeaponPack/Blueprints/InventorySlot_Struct` null))
    (`self.UpdateSlotAtIndex` (`local.LocalIndex`))
    (return true)
    (else
      (return false))))

(fn `SearchEmptySlot`
  (returns (Success :type Boolean) (Index :type Integer))
  (locals (LocalIndex :type Integer) (LocalBool :type Boolean))
  (for (_array_element _array_index) (`self.Slots`)
    (if (not (`KismetSystemLibrary.IsValidClass` (`.ItemClass_3_A40736744D9AD799DC31BD8DDFCB6A7A` (break `/Game/AdvanceWeaponPack/Blueprints/InventorySlot_Struct` _array_element))))
      (set `local.LocalBool` true)
      (set `local.LocalIndex` _array_index)
      (break)))
  (return (`local.LocalBool`) (`local.LocalIndex`)))

(fn `SearchFreeStack`
  (params (ItemClass :type "/Game/AdvanceWeaponPack/Blueprints/Attachment/BP_BaseAttachment_BP Class Reference"))
  (returns (`Success?` :type Boolean) (Indes :type Integer))
  (locals (LocalIndex :type Integer) (LocalBool :type Boolean))
  (for (_array_element _array_index) (`self.Slots`)
    (bind _itemclass (break `/Game/AdvanceWeaponPack/Blueprints/InventorySlot_Struct` _array_element))
    (if (`KismetSystemLibrary.IsValidClass` _itemclass)
      (if (== ItemClass _itemclass)
        (set `local.LocalBool` true)
        (set `local.LocalIndex` _array_index)
        (break))))
  (return (`local.LocalBool`) (`local.LocalIndex`)))

(fn `SwapSlots`
  (params (Index1 :type Integer) (Index2 :type Integer))
  (returns (`Success?` :type Boolean))
  (locals (LocalIndex1 :type Integer) (LocalIndex2 :type Integer) (LocalSlot2 :type "/Game/AdvanceWeaponPack/Blueprints/InventorySlot_Struct Structure"))
  (bind _localindex2 (`local.LocalIndex2`))
  (bind _slots (`self.Slots`))
  (bind _returnvalue (`KismetArrayLibrary.Array_LastIndex` (`self.Slots`)))
  (set `local.LocalIndex1` Index1)
  (set `local.LocalIndex2` Index2)
  (if (or (> (`local.LocalIndex1`) _returnvalue) (> _returnvalue (`local.LocalIndex2`)))
    (set `local.LocalSlot2` (`|GetArrayItem` _slots _localindex2))
    (`KismetArrayLibrary.Array_Set` _slots _localindex2 (`|GetArrayItem` (`self.Slots`) (`local.LocalIndex1`)))
    (`KismetArrayLibrary.Array_Set` (`self.Slots`) (`local.LocalIndex1`) (`local.LocalSlot2`))
    (`self.UpdateSlotAtIndex` (`local.LocalIndex1`))
    (`self.UpdateSlotAtIndex` (`local.LocalIndex2`))
    (return true)
    (else
      (return false))))

(fn `UserConstructionScript`)