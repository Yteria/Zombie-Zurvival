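; Modular mounted ladder whose height follows a LadderHeight gizmo, flagging FirstPersonCharacter for climbing.
; The construction script steps the mid-segment count in 100-unit increments, then chains meshes between bottom and top via sockets.
; It optionally adds rung joints and a top cover, then fits the trigger box to the ladder.
; Box overlap sets PlayerNearLadder; leaving clears near and on-ladder flags and restores walking.
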(event `self.Box.OnComponentBeginOverlap`
  (params (OverlappedComponent :type "PrimitiveComponent Object Reference") (OtherActor :type "Actor Object Reference") (OtherComp :type "PrimitiveComponent Object Reference") (OtherBodyIndex :type Integer) (bFromSweep :type Boolean) (SweepResult :type "HitResult Structure (by ref)"))
  (bind _asfirst_person_character (cast `/Game/ZombieZurvival/MOUT_Fabrication/Demo/FirstPersonBP/Blueprints/FirstPersonCharacter` OtherActor))
  (set `/Game/ZombieZurvival/MOUT_Fabrication/Demo/FirstPersonBP/Blueprints/FirstPersonCharacter.PlayerNearLadder?` true _asfirst_person_character))

(event `self.Box.OnComponentEndOverlap`
  (params (OverlappedComponent :type "PrimitiveComponent Object Reference") (OtherActor :type "Actor Object Reference") (OtherComp :type "PrimitiveComponent Object Reference") (OtherBodyIndex :type Integer))
  (bind _asfirst_person_character (cast `/Game/ZombieZurvival/MOUT_Fabrication/Demo/FirstPersonBP/Blueprints/FirstPersonCharacter` OtherActor))
  (set `/Game/ZombieZurvival/MOUT_Fabrication/Demo/FirstPersonBP/Blueprints/FirstPersonCharacter.PlayerNearLadder?` false _asfirst_person_character)
  (set `/Game/ZombieZurvival/MOUT_Fabrication/Demo/FirstPersonBP/Blueprints/FirstPersonCharacter.PlayerOnLadder?` false _asfirst_person_character)
  (`CharacterMovementComponent.SetMovementMode` (`Character.CharacterMovement` _asfirst_person_character) "MOVE_Walking" 0))

(fn `UserConstructionScript`
  (locals (TransformDown :type "Transform Structure" :default "0.000000,0.000000,-100.000000|0.000000,0.000000,0.000000|1.000000,1.000000,1.000000"))
  (bind _addedcoversegments (`self.AddedCoverSegments`))
  (bind _addedladdersegments (`self.AddedLadderSegments`))
  (bind _addedcoversegments_2 (`self.AddedCoverSegments`))
  (bind _addedladdersegments_2 (`self.AddedLadderSegments`))
  (bind _box (`self.Box`))
  (bind _addedladdersegments_3 (`self.AddedLadderSegments`))
  (bind _z (.z (`self.LadderHeight`)))
  ;[1 1 1] Default to No Height
  (`SceneComponent.K2_AttachToComponent` (`self.TopLadder`) (`self.BottomLadder`) "NextConnector" "KeepRelative" "KeepRelative" "KeepRelative" true)
  (`|ExecutionSequence`
    (:`then_0`
      ;[1 1 1] Get LadderHeight Gizmo and Convert into Integers for Mid Section Generation
      (set `self.HeightFloat` _z)
      (if (> _z (+ (`self.AdditionHeightFloat`) 100.0))
        (set `self.LadderAdjusted` true)
        (set `self.AdditionHeightFloat` (+ (`self.AdditionHeightFloat`) 100.0))
        (set `self.NumberOfLadderSegments` (+ (`self.NumberOfLadderSegments`) 1))
        (elif (< (`self.HeightFloat`) (`self.AdditionHeightFloat`))
          (set `self.AdditionHeightFloat` (+ (`self.AdditionHeightFloat`) -100.0))
          (set `self.NumberOfLadderSegments` (+ (`self.NumberOfLadderSegments`) -1)))))
    (:`then_1`
      ;[1 1 1] Add Mid Sections to Ladders
      (`KismetArrayLibrary.Array_Clear` (`self.AddedLadderSegments`))
      (for _ (range (+ (`self.NumberOfLadderSegments`) 1))
        (bind _returnvalue (`AddComponent|NODE_AddStaticMeshComponent-2` :`bManualAttachment` true))
        (bind _returnvalue_2 (`KismetArrayLibrary.Array_Add` _addedladdersegments_3 _returnvalue))
        (`SceneComponent.K2_AttachToComponent` _returnvalue (`|GetArrayItem` _addedladdersegments_3 (- _returnvalue_2 1)) "NextConnector" "KeepRelative" "KeepRelative" "KeepRelative" true))
      (`SceneComponent.K2_AttachToComponent` (`self.TopLadder`) (`|GetArrayItem` _addedladdersegments (`KismetArrayLibrary.Array_LastIndex` _addedladdersegments)) "NextConnector" "SnapToTarget" "SnapToTarget" "SnapToTarget" true)
      (`SceneComponent.K2_AttachToComponent` (`|GetArrayItem` (`self.AddedLadderSegments`)) (`self.BottomLadder`) "NextConnector" "KeepRelative" "KeepRelative" "KeepRelative" true))
    (:`then_2`
      ;[1 1 1] Add Rung Joints
      (if (`self.AddRungs`)
        (for (_ _array_index) _addedladdersegments_2
          (bind _returnvalue_3 (`AddComponent|NODE_AddStaticMeshComponent-5`))
          (`SceneComponent.K2_AttachToComponent` _returnvalue_3 (`|GetArrayItem` _addedladdersegments_2 _array_index) "MainConnector" "KeepRelative" "KeepRelative" "KeepRelative" true))))
    (:`then_3`
      ;[1 1 1] Add Ladder Top Cover / Protectors
      (if (`self.AddTopCover`)
        (bind _returnvalue_4 (`AddComponent|NODE_AddStaticMeshComponent-6` :`bManualAttachment` true :`RelativeTransform` (`self.Top Cover Transform`)))
        (bind _output_get (set `self.TopCover` _returnvalue_4))
        (`SceneComponent.K2_AttachToComponent` _output_get (`self.TopLadder`) "EndConnector" "KeepRelative" "KeepRelative" "KeepRelative" true)
        (`KismetArrayLibrary.Array_Clear` (`self.AddedCoverSegments`))
        (for _ (range (+ (- (`self.NumberOfLadderSegments`) 2) 1))
          (bind _returnvalue_5 (`AddComponent|NODE_AddStaticMeshComponent-16` :`bManualAttachment` true :`RelativeTransform` (`local.TransformDown`)))
          (bind _returnvalue_6 (`KismetArrayLibrary.Array_Add` _addedcoversegments _returnvalue_5))
          (`SceneComponent.K2_AttachToComponent` _returnvalue_5 (`|GetArrayItem` _addedcoversegments (- _returnvalue_6 1)) "EndConnector" "KeepRelative" "KeepRelative" "KeepRelative" true))
        (`SceneComponent.K2_AttachToComponent` (`|GetArrayItem` _addedcoversegments_2 (`KismetArrayLibrary.Array_LastIndex` _addedcoversegments_2)) (`self.TopCover`) "EndCover" "KeepRelative" "KeepRelative" "KeepRelative" true)
        (`SceneComponent.K2_AttachToComponent` (`|GetArrayItem` (`self.AddedCoverSegments`)) (`self.TopCover`) "EndCover" "KeepRelative" "KeepRelative" "KeepRelative" true)))
    (:`then_4`
      ;[1 1 1] Auto Collision Generation
      (`BoxComponent.SetBoxExtent` _box (`.BoxExtent` (`self.GetActorBounds` true true)) true)
      (`SceneComponent.K2_SetWorldLocation` _box (/ (+ (`SceneComponent.K2_GetComponentLocation` (`self.BottomLadderBoundsRef`)) (+ (`SceneComponent.K2_GetComponentLocation` (`self.TopLadderBoundsRef`)) (0.0 0.0 50.0))) 2.0) false false))))