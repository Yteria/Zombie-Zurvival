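; BP_EnemySpawner is a spawner actor that spawns queued enemy classes at its own transform.
; AddEnemyToQueue appends a class and immediately spawns the front of the queue if no BP_Enemy overlaps its Sphere.
; A looping timer from BeginPlay also spawns the next queued enemy every two seconds, without that overlap check.
; OnEnemyDefeated only casts to BP_GameMode_ZZ and takes no further action.
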(event `OnEnemyDefeated`
  (cast `/Game/Workspaces/Elliott/BP_GameMode_ZZ` (`GameplayStatics.GetGameMode`)))

(event `self.ReceiveBeginPlay`
  (`KismetSystemLibrary.K2_SetTimerDelegate` (delegate `TryToSpawn`) 2.0 true))

(event `TryToSpawn`
  (`self.SpawnEnemy`))

(fn `AddEnemyToQueue`
  (params (EnemyClass :type "/Game/Workspaces/Elliott/Zombie2/BP_Enemy Class Reference (by ref)"))
  (`KismetArrayLibrary.Array_Add` (`self.EnnemyQueue`) EnemyClass)
  (if (not (`KismetArrayLibrary.Array_IsValidIndex` (`PrimitiveComponent.GetOverlappingActors` (`self.Sphere`) "/Game/Workspaces/Elliott/Zombie2/BP_Enemy.BP_Enemy_C")))
    (`self.SpawnEnemy`)))

(fn `SpawnEnemy`
  (returns (Succes :type Boolean))
  (if (`KismetArrayLibrary.Array_IsValidIndex` (`self.EnnemyQueue`))
    (`|SpawnActorFromClass` (`|GetArrayItem` (`self.EnnemyQueue`)) (`self.GetTransform`) "AdjustIfPossibleButAlwaysSpawn" "MultiplyWithRoot" null null)
    (`KismetArrayLibrary.Array_Remove` (`self.EnnemyQueue`))
    (return true)
    (else
      (return false))))

(fn `UserConstructionScript`)