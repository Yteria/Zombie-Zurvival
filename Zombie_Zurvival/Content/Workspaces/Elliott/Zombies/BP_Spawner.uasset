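; BP_Spawner is a zombie-mode enemy spawner that queues enemy classes and spawns them at its own transform.
; Queued classes spawn immediately if no BP_Zombi1 overlaps its sphere, while a looping timer also spawns from the queue head without that check.
; Each spawn receives Health and Damage through a stats message and gets a destruction binding, with a defeat event that notifies BP_GameMode_ZZ.
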(event `self.ReceiveBeginPlay`
  (`KismetSystemLibrary.K2_SetTimerDelegate` (delegate `TryTooSpawn`) 2.0 true))

(event `TryTooSpawn`
  (`self.SpawnEnemy`))

(event `OnEnemyDefeated`
  (bind _asbp_game_mode_zz (cast `/Game/Workspaces/Elliott/BP_GameMode_ZZ` (`GameplayStatics.GetGameMode`)))
  (`/Game/Workspaces/Elliott/BP_GameMode_ZZ.OnEnemyDefeated` _asbp_game_mode_zz))

(fn `AddEnemyToQueue`
  (params (EnemyClass :type "/Game/Workspaces/Elliott/Zombies/BP_Zombi1 Class Reference (by ref)"))
  (`KismetArrayLibrary.Array_Add` (`self.EnemyQueue`) EnemyClass)
  (if (not (`KismetArrayLibrary.Array_IsValidIndex` (`PrimitiveComponent.GetOverlappingActors` (`self.Sphere`) "/Game/Workspaces/Elliott/Zombies/BP_Zombi1.BP_Zombi1_C")))
    (`self.SpawnEnemy`)))

(fn `SpawnEnemy`
  (returns (Succes :type Boolean))
  (if (`KismetArrayLibrary.Array_IsValidIndex` (`self.EnemyQueue`))
    (bind _returnvalue (`|SpawnActorFromClass` (`|GetArrayItem` (`self.EnemyQueue`)) (`self.GetTransform`) "AdjustIfPossibleButAlwaysSpawn" "MultiplyWithRoot" null null))
    (add `/Game/Workspaces/Elliott/Zombies/BP_Zombi1.WhenDestroyed` _returnvalue (`|CreateDelegate` :!event `OnEnemyDefeated`))
    (message `/Game/Workspaces/Anton/BPI_Enemy_Stats.EnemyStats` _returnvalue (`self.Health`) (`self.Damage`))
    (`KismetArrayLibrary.Array_Remove` (`self.EnemyQueue`))
    (return true)
    (else
      (return false))))

(fn `UserConstructionScript`)