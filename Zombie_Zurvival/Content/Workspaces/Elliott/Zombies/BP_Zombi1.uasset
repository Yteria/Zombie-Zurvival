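; BP_Zombi1 is a zombie enemy that chases the player and damages them on overlap with its Damage component.
; It moves through both SimpleMoveToActor every Tick and an AIMoveTo loop from BeginPlay that repeats three seconds after success.
; The first Tick copies EnemyStats values into health and damage.
; Incoming damage lowers health, prints it, and destroys the zombie at zero.
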(event `/Game/Workspaces/Anton/BPI_Enemy_Stats.EnemyStats`
  (params (Health :type "Float (double-precision)") (Damage :type "Float (double-precision)")))

(event `self.ReceiveTick`
  (params (DeltaSeconds :type "Float (single-precision)"))
  (`|ExecutionSequence`
    (:`then_0`
      (`/Engine/EditorBlueprintResources/StandardMacros.DoOnce` false
        (:`Completed`
          (set `self.Health` (stale `/Game/Workspaces/Anton/BPI_Enemy_Stats.EnemyStats` Health))
          (set `self.Dmg` (stale `/Game/Workspaces/Anton/BPI_Enemy_Stats.EnemyStats` Damage)))))
    (:`then_1`
      (`AIBlueprintHelperLibrary.SimpleMoveToActor` (`self.GetController`) (`GameplayStatics.GetPlayerCharacter` 0)))))

(event `Move`
  (`|AIMoveTo` self (0.0 0.0 0.0) (`GameplayStatics.GetPlayerCharacter` 0)
    (:`OnSuccess`
      (`KismetSystemLibrary.Delay` 3.0)
      (`self.Move`))))

(event `self.ReceiveBeginPlay`
  (`self.Move`))

(event `self.ReceiveAnyDamage`
  (params (Damage :type "Float (single-precision)") (DamageType :type "DamageType Object Reference") (InstigatedBy :type "Controller Object Reference") (DamageCauser :type "Actor Object Reference"))
  (bind _output_get (set `self.Health` (- (`self.Health`) Damage)))
  (`KismetSystemLibrary.PrintString` (`KismetStringLibrary.Conv_DoubleToString` _output_get) true true (struct :`G` 1.0 :`B` 0.033423 :`A` 1.0))
  (if (<= (`self.Health`) 0.0)
    (`self.K2_DestroyActor`)))

(event `self.Damage.OnComponentBeginOverlap`
  (params (OverlappedComponent :type "PrimitiveComponent Object Reference") (OtherActor :type "Actor Object Reference") (OtherComp :type "PrimitiveComponent Object Reference") (OtherBodyIndex :type Integer) (bFromSweep :type Boolean) (SweepResult :type "HitResult Structure (by ref)"))
  (if (== OtherActor (`GameplayStatics.GetPlayerPawn` 0))
    (`GameplayStatics.ApplyDamage` OtherActor (`self.Dmg`))))

(fn `UserConstructionScript`)